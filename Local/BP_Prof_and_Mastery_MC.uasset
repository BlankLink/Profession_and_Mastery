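; Mod controller for a professions and class mastery mod that injects the mod's content into the game's data tables.
; ModDataTableOperations merges custom tables into feats, items, recipes, profession templates, equipment variations and eye and lip makeup colors.
; Several merges layer stat overwrites, including DLC and primal sets, onto the item stat modification table.
; The construction script and Widget function are empty, and a few leftover merge calls are unconnected.
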(fn ConstructionScript)

(fn ModDataTableOperations
  (Class|ModController|MergeDataTables "/Game/Items/Feats/FeatTable.FeatTable" "/Game/Mods/Profession_and_Mastery/DataTables/dt_Feat_Table.dt_Feat_Table")
  (Class|ModController|MergeDataTables "/Game/Items/ItemTable.ItemTable" "/Game/Mods/Profession_and_Mastery/DataTables/dt_Class_Mastery_Item_Table.dt_Class_Mastery_Item_Table")
  (Class|ModController|MergeDataTables "/Game/Items/Recipes/RecipesTable.RecipesTable" "/Game/Mods/Profession_and_Mastery/DataTables/dt_Class_Mastery_Recipe_Table.dt_Class_Mastery_Recipe_Table")
  (Class|ModController|MergeDataTables "/Game/Systems/SpawnTable/ProfessionTemplateDataTable.ProfessionTemplateDataTable" "/Game/Mods/Profession_and_Mastery/DataTables/dt_Profession_Template_Table.dt_Profession_Template_Table")
  (Class|ModController|MergeDataTables "/Game/Items/ItemStatModificationTable.ItemStatModificationTable" "/Game/Mods/Profession_and_Mastery/DataTables/dt_custom_item_modif.dt_custom_item_modif")
  (Class|ModController|MergeDataTables "/Game/Items/EquipmentVariationTable.EquipmentVariationTable" "/Game/Mods/Profession_and_Mastery/DataTables/dt_custom_equip_var.dt_custom_equip_var")
  (Class|ModController|MergeDataTables "/Game/Items/ItemStatModificationTable.ItemStatModificationTable" "/Game/Mods/Profession_and_Mastery/DataTables/dt_OW_ItemStatModificationTable.dt_OW_ItemStatModificationTable")
  (Class|ModController|MergeDataTables "/Game/UI/CharacterCreation/DataTables/EyeMakeupColorSelections.EyeMakeupColorSelections" "/Game/Mods/Profession_and_Mastery/DataTables/dt_corrupted_colours.dt_corrupted_colours")
  (Class|ModController|MergeDataTables "/Game/UI/CharacterCreation/DataTables/LipMakeupColorSelections.LipMakeupColorSelections" "/Game/Mods/Profession_and_Mastery/DataTables/dt_corrupted_colours.dt_corrupted_colours")
  (Class|ModController|MergeDataTables "/Game/Items/ItemStatModificationTable.ItemStatModificationTable" "/Game/Mods/Profession_and_Mastery/DataTables/dt_OW_DLC_ItemStatModificationTable.dt_OW_DLC_ItemStatModificationTable")
  (Class|ModController|MergeDataTables "/Game/Items/ItemStatModificationTable.ItemStatModificationTable" "/Game/Mods/Profession_and_Mastery/DataTables/dt_Primal_Stat_Overwrite.dt_Primal_Stat_Overwrite")
  (Class|ModController|MergeDataTables "/Game/Items/ItemStatModificationTable.ItemStatModificationTable" "/Game/Mods/Profession_and_Mastery/DataTables/dt_OW_DLC3_ItemStatModificationTable.dt_OW_DLC3_ItemStatModificationTable")
  (Class|ModController|MergeDataTables "/Game/Items/ItemStatModificationTable.ItemStatModificationTable" "/Game/Mods/Profession_and_Mastery/DataTables/dt_OW_DLC4_ItemStatModificationTable.dt_OW_DLC4_ItemStatModificationTable")
  (Class|ModController|MergeDataTables "/Game/Items/ItemStatModificationTable.ItemStatModificationTable" "/Game/Mods/Profession_and_Mastery/DataTables/dt_OW_DLC2_ItemStatModificationTable.dt_OW_DLC2_ItemStatModificationTable"))

(fn Widget)