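; Usable lockpick item that lets a player unlock a traced door, hatch or container while its owner or guild is online.
; CheckDifficulty rates the target by class and display name, then buffs and a tinkering emote cover timed delays.
; RollUnlock rolls d100 against difficulty, class-based skill and data-table item tier.
; Movement velocity changes or damage interrupt picking; success, failure and interruption all apply an exhaustion buff.
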(event Custom|CustomEvent_0
  (params (DeltaSeconds :type Float%20%28single-precision%29) (OldLocation :type Vector) (OldVelocity :type Vector))
  (bind _invokingbaseplayer (Variables|Default|GetInvokingBasePlayer))
  (bind _invokingbaseplayer_2 (Variables|Default|GetInvokingBasePlayer))
  (bind _invokingbaseplayer_3 (Variables|Default|GetInvokingBasePlayer))
  (if (not (Math|Vector|Equal(Vector) (- (Transformation|GetVelocity _invokingbaseplayer) OldVelocity) "0, 0, 0" 0.0001))
    (Default|EndBuff (Variables|/Game/Characters/BaseBPCombat.BaseBPCombat_C|Get00_BP_AC_BuffSystem _invokingbaseplayer) "/Game/Mods/Profession_and_Mastery/System/Buffs/BP_AC_Buff_Lockpick.BP_AC_Buff_Lockpick_C")
    (Default|EffectstoPlay (Actor|GetComponentbyClass (Variables|Default|GetInvokingBasePlayer) "/Game/Mods/Profession_and_Mastery/AC_Actor_Component_Main.AC_Actor_Component_Main_C") "/Game/Characters/humans/animations/emotes/AM_emote_tinkering.AM_emote_tinkering" false 0 0 "0, 0, 0")
    (Class|HUDNotificationInterface|NotificationText(Message) (CallFunction|GetControllerfromActor (Variables|Default|GetInvokingBasePlayer)) "Lockpicking interrupted!" false)
    (Variables|Default|SetUnlockTarget 0)
    (Default|AddBuff (Variables|/Game/Characters/BaseBPCombat.BaseBPCombat_C|Get00_BP_AC_BuffSystem _invokingbaseplayer_2) "/Game/Mods/Profession_and_Mastery/System/Buffs/BP_Exhaustion_Lockpick.BP_Exhaustion_Lockpick_C" _invokingbaseplayer_2)
    (EventDispatchers|UnbindEventfromOnTakeAnyDamage _invokingbaseplayer_3 (delegate Custom|Interrupt%20by%20damage%20taken))
    (Character|UnbindEventfromOnCharacterMovementUpdated _invokingbaseplayer_3 (delegate Custom|CustomEvent_0))))

(event Custom|Interrupt%20by%20damage%20taken
  (params (DamagedActor :type Actor%20Object%20Reference) (Damage :type Float%20%28single-precision%29) (DamageType :type Damage%20Type%20Object%20Reference) (InstigatedBy :type Controller%20Object%20Reference) (DamageCauser :type Actor%20Object%20Reference) (DamageEventID :type Integer))
  (bind _invokingbaseplayer (Variables|Default|GetInvokingBasePlayer))
  (bind _invokingbaseplayer_2 (Variables|Default|GetInvokingBasePlayer))
  (Default|EndBuff (Variables|/Game/Characters/BaseBPCombat.BaseBPCombat_C|Get00_BP_AC_BuffSystem (Variables|Default|GetInvokingBasePlayer)) "/Game/Mods/Profession_and_Mastery/System/Buffs/BP_AC_Buff_Lockpick.BP_AC_Buff_Lockpick_C")
  (Default|EffectstoPlay (Actor|GetComponentbyClass (Variables|Default|GetInvokingBasePlayer) "/Game/Mods/Profession_and_Mastery/AC_Actor_Component_Main.AC_Actor_Component_Main_C") "/Game/Characters/humans/animations/emotes/AM_emote_tinkering.AM_emote_tinkering" false 0 0 "0, 0, 0")
  (Class|HUDNotificationInterface|NotificationText(Message) (CallFunction|GetControllerfromActor (Variables|Default|GetInvokingBasePlayer)) "Lockpicking interrupted!" false)
  (Variables|Default|SetUnlockTarget 0)
  (Default|AddBuff (Variables|/Game/Characters/BaseBPCombat.BaseBPCombat_C|Get00_BP_AC_BuffSystem _invokingbaseplayer) "/Game/Mods/Profession_and_Mastery/System/Buffs/BP_Exhaustion_Lockpick.BP_Exhaustion_Lockpick_C" _invokingbaseplayer)
  (EventDispatchers|UnbindEventfromOnTakeAnyDamage _invokingbaseplayer_2 (delegate Custom|Interrupt%20by%20damage%20taken))
  (Character|UnbindEventfromOnCharacterMovementUpdated _invokingbaseplayer_2 (delegate Custom|CustomEvent_0)))

(event EventOnUseItem
  (params (invokingCharacter :type Conan%20Character%20Object%20Reference))
  (bind _asbase_player_char (Utilities|Casting|CastToBasePlayerChar invokingCharacter))
  (bind _output_get (Variables|Default|SetInvokingBasePlayer _asbase_player_char))
  (Utilities|SetSkillLevel _output_get)
  (bind _outhit (Collision|SphereTraceForObjects (+ (Transformation|GetSocketLocation (Actor|GetComponentbyClass _output_get "/Script/Engine.SkeletalMeshComponent") "b_head") "0, 0,10.000000") (- (+ (* (Math|Vector|GetRightVector (Actor|GetComponentbyClass _output_get "/Script/Engine.SkeletalMeshComponent")) 160) (Transformation|GetSocketLocation (Actor|GetComponentbyClass _output_get "/Script/Engine.SkeletalMeshComponent") "b_head")) "0, 0,130.000000") 0.0 (Utilities|Array|MakeArray "ObjectTypeQuery2" "ObjectTypeQuery10") false (Utilities|Array|MakeArray _asbase_player_char) "None"))
  (bind _asbp_master_placeables (Utilities|Casting|CastToBP_Master_Placeables (.hitactor _outhit))
    (:then
      (bind _false (CallFunction|CheckDifficulty _asbp_master_placeables))
      (if _false
        (bind _online (CallFunction|CheckOwnerOnline (Variables|Default|GetUnlockTarget)))
        (if _online
          (Default|EffectstoPlay (Actor|GetComponentbyClass (Variables|Default|GetInvokingBasePlayer) "/Game/Mods/Profession_and_Mastery/AC_Actor_Component_Main.AC_Actor_Component_Main_C") "/Game/Characters/humans/animations/emotes/AM_emote_tinkering.AM_emote_tinkering" true 0 0 "0, 0, 0")
          (Default|AddBuff (Variables|/Game/Characters/BaseBPCombat.BaseBPCombat_C|Get00_BP_AC_BuffSystem (Variables|Default|GetInvokingBasePlayer)) "/Game/Mods/Profession_and_Mastery/System/Buffs/BP_AC_Buff_Lockpick.BP_AC_Buff_Lockpick_C" (Variables|Default|GetInvokingBasePlayer))
          (EventDispatchers|BindEventtoOnTakeAnyDamage (Variables|Default|GetInvokingBasePlayer) (delegate Custom|Interrupt%20by%20damage%20taken))
          (Character|BindEventtoOnCharacterMovementUpdated (Variables|Default|GetInvokingBasePlayer) (delegate Custom|CustomEvent_0))
          (Utilities|FlowControl|Delay 15.0)
          (Utilities|RollUnlock
            (:Success
              (Class|FuncomGenericLibrary|LogGameEvent 0 "INFOL_INFO0" "Lock Picked")
              (Utilities|FlowControl|Delay 15.0)
              (if (.HasBuff (Default|CheckifBuffExists (Variables|/Game/Characters/BaseBPCombat.BaseBPCombat_C|Get00_BP_AC_BuffSystem (Variables|Default|GetInvokingBasePlayer)) "/Game/Mods/Profession_and_Mastery/System/Buffs/BP_AC_Buff_Lockpick.BP_AC_Buff_Lockpick_C"))
                (if (Variables|Default|GetPIPPI)
                  (Default|CustomInteraction (Variables|Default|GetUnlockTarget) 0 1234 false)
                  (else
                    (Default|SetLockedState (Variables|Default|GetUnlockTarget) false)))
                (Default|EndBuff (Variables|/Game/Characters/BaseBPCombat.BaseBPCombat_C|Get00_BP_AC_BuffSystem (Variables|Default|GetInvokingBasePlayer)) "/Game/Mods/Profession_and_Mastery/System/Buffs/BP_AC_Buff_Lockpick.BP_AC_Buff_Lockpick_C")
                (Class|AudioFunctionLibrary|PlaySoundatLocation "/Game/Sound/SFX/Gui/gui_unlock_item_3.gui_unlock_item_3" (Transformation|GetActorLocation (Variables|Default|GetInvokingBasePlayer)))
                (Default|EffectstoPlay (Actor|GetComponentbyClass (Variables|Default|GetInvokingBasePlayer) "/Game/Mods/Profession_and_Mastery/AC_Actor_Component_Main.AC_Actor_Component_Main_C") "/Game/Characters/humans/animations/emotes/AM_emote_tinkering.AM_emote_tinkering" false 0 0 "0, 0, 0")
                (Variables|Default|SetUnlockTarget 0)
                (Default|AddBuff (Variables|/Game/Characters/BaseBPCombat.BaseBPCombat_C|Get00_BP_AC_BuffSystem (Variables|Default|GetInvokingBasePlayer)) "/Game/Mods/Profession_and_Mastery/System/Buffs/BP_Exhaustion_Lockpick.BP_Exhaustion_Lockpick_C" (Variables|Default|GetInvokingBasePlayer) :!label _label)
                (EventDispatchers|UnbindEventfromOnTakeAnyDamage (Variables|Default|GetInvokingBasePlayer) (delegate Custom|Interrupt%20by%20damage%20taken) :!label _label_2)
                (Character|UnbindEventfromOnCharacterMovementUpdated (Variables|Default|GetInvokingBasePlayer) (delegate Custom|CustomEvent_0))))
            (:Failure
              (Default|EndBuff (Variables|/Game/Characters/BaseBPCombat.BaseBPCombat_C|Get00_BP_AC_BuffSystem (Variables|Default|GetInvokingBasePlayer)) "/Game/Mods/Profession_and_Mastery/System/Buffs/BP_AC_Buff_Lockpick.BP_AC_Buff_Lockpick_C")
              (Default|EffectstoPlay (Actor|GetComponentbyClass (Variables|Default|GetInvokingBasePlayer) "/Game/Mods/Profession_and_Mastery/AC_Actor_Component_Main.AC_Actor_Component_Main_C") "/Game/Characters/humans/animations/emotes/AM_emote_tinkering.AM_emote_tinkering" false 0 0 "0, 0, 0")
              (Class|HUDNotificationInterface|NotificationText(Message) (CallFunction|GetControllerfromActor (Variables|Default|GetInvokingBasePlayer)) "The lockpick broke" false)
              (Variables|Default|SetUnlockTarget 0)
              (if (> (Math|Random|RandomIntegerinRange 0 100) 49)
                (|CallParentFunction invokingCharacter)
                (goto _label)
                (else
                  (goto _label)))))
          (elif (Networking|IsServer)
            ;[1 0 0] checkonline
            (Class|HUDNotificationInterface|NotificationText(Message) (CallFunction|GetControllerfromActor (Variables|Default|GetInvokingBasePlayer)) "Something feels wrong about this" false)
            (goto _label_2)
            (else
              (goto _label_2))))
        (else
          (Class|HUDNotificationInterface|NotificationText(Message) (CallFunction|GetControllerfromActor (Variables|Default|GetInvokingBasePlayer)) "Couldn't find a valid target" false :!label _label_3))))
    (:CastFailed
      (goto _label_3))))

(fn CheckOwnerOnline
  (params (BuildingPart :type Buildable%20Base%20Object%20Reference))
  (bind _invokingbaseplayer (Variables|Default|GetInvokingBasePlayer))
  (bind _returnvalue (Actor|GetComponentbyClass _invokingbaseplayer "/Game/Mods/Profession_and_Mastery/AC_Actor_Component_Main.AC_Actor_Component_Main_C"))
  (bind _returnvalue_2 (Class|FuncomGenericLibrary|GetCharacterfromUniqueId (Variables|/Script/ConanSandbox.BuildableBase|GetOwnerUniqueID BuildingPart)))
  (Utilities|IsValid (Pawn|GetController _returnvalue_2)
    (:Is%20Valid
      (bind _output_get (Variables|Default|SetOwnerOnline true))
      (return _output_get))
    (:Is%20Not%20Valid
      (Default|RefreshOnlineGuildList _returnvalue)
      (bind _returnvalue_3 (Class|BuildableBase|GetOwnerName BuildingPart))
      (if (>= (Utilities|Array|FindItem (Variables|/Game/Mods/Profession_and_Mastery/AC_Actor_Component_Main.AC_Actor_Component_Main_C|GetOnlineGuildNameList _returnvalue) (Utilities|String|ToString(Text) _returnvalue_3)) 0)
        (bind _output_get_2 (Variables|Default|SetOwnerOnline true))
        (return _output_get_2)
        (else
          (Variables|Default|SetOwnerOnline false)
          (return false))))))

(fn CheckDifficulty
  (params (Object :type Object%20Object%20Reference))
  (if (> (Utilities|String|FindSubstring (Utilities|GetDisplayName (Variables|Default|GetUnlockTarget)) "egress") -1)
    (Variables|Default|SetPIPPI true)
    (Variables|Default|SetLockDifficulty 2)
    (return true)
    (elif (> (Utilities|String|FindSubstring (Utilities|GetDisplayName (Variables|Default|GetUnlockTarget)) "nomad") -1)
      (Variables|Default|SetLockDifficulty 3)
      (return true)
      (else
        (bind _asbp_master_placeables (Utilities|Casting|CastToBP_Master_Placeables Object)
          (:then
            (bind _output_get (Variables|Default|SetUnlockTarget _asbp_master_placeables))
            (Utilities|Casting|CastToBP_PL_Door _output_get
              (:then
                (Utilities|Casting|CastToBP_PL_GateDoor (Variables|Default|GetUnlockTarget)
                  (:then
                    (Variables|Default|SetLockDifficulty 0)
                    (return false))
                  (:CastFailed
                    _)))
              (:CastFailed
                (Utilities|Casting|CastToBP_PL_Hatch (Variables|Default|GetUnlockTarget)
                  (:then
                    _)
                  (:CastFailed
                    (Utilities|Casting|CastToBP_PL_Chest_Large (Variables|Default|GetUnlockTarget)
                      (:then
                        (Variables|Default|SetLockDifficulty 2))
                      (:CastFailed
                        (Utilities|Casting|CastToBP_PL_Chest_Vault (Variables|Default|GetUnlockTarget)
                          (:then
                            (Variables|Default|SetLockDifficulty 0)
                            (return false))
                          (:CastFailed
                            (Utilities|Casting|CastToBP_PlaceableItemContainer (Variables|Default|GetUnlockTarget)
                              (:then
                                (Variables|Default|SetLockDifficulty 1))
                              (:CastFailed
                                (Variables|Default|SetLockDifficulty 0)))))))
                    (return true)))))
            (if (Utilities|String|Contains (Utilities|GetDisplayName (Variables|Default|GetUnlockTarget)) "T1" false true)
              (Variables|Default|SetLockDifficulty 1)
              (elif (Utilities|String|Contains (Utilities|GetDisplayName (Variables|Default|GetUnlockTarget)) "T2" false true)
                (Variables|Default|SetLockDifficulty 2)
                (elif (Utilities|String|Contains (Utilities|GetDisplayName (Variables|Default|GetUnlockTarget)) "T3" false true)
                  (Variables|Default|SetLockDifficulty 3)
                  (else
                    (return false)))))
            (return true))
          (:CastFailed
            (Variables|Default|SetLockDifficulty 0)
            (return false)))))))